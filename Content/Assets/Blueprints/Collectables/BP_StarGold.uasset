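; BP_StarGold is a collectable gold star that the player and fake players can take.
; Each tick it spins the star mesh by interpolating yaw toward an offset from its current value.
; On trigger overlap, BP_CubePlayer adds a star and score through GM_ToxBoxInGame with a randomly pitched sound.
; A BP_FakePlayer instead plays its win animation and deducts score; either pickup destroys the star.
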(event `self.ReceiveTick`
  (params (DeltaSeconds :type "Float (single-precision)"))
  (set `self.Delta Seconds` DeltaSeconds)
  (`self.TurnAnimation`))

(event `TurnAnimation`
  (bind _star (`self.Star`))
  (bind (_returnvalue_roll _returnvalue_pitch _returnvalue_yaw) (`KismetMathLibrary.BreakRotator` (`SceneComponent.K2_GetComponentRotation` _star)))
  (`SceneComponent.K2_SetWorldRotation` _star (`KismetMathLibrary.MakeRotator` _returnvalue_roll _returnvalue_pitch (`KismetMathLibrary.FInterpTo` _returnvalue_yaw (+ _returnvalue_yaw 20.0) (`self.Delta Seconds`) 5.0)) false false))

(event `self.Trigger.OnComponentBeginOverlap`
  (params (OverlappedComponent :type "PrimitiveComponent Object Reference") (OtherActor :type "Actor Object Reference") (OtherComp :type "PrimitiveComponent Object Reference") (OtherBodyIndex :type Integer) (bFromSweep :type Boolean) (SweepResult :type "HitResult Structure (by ref)"))
  (cast `/Game/Assets/Blueprints/Players/BP_CubePlayer` OtherActor
    (:`then`
      (bind _asgm_tox_box_in_game (cast `/Game/Assets/Blueprints/GameManager/GM_ToxBoxInGame` (`GameplayStatics.GetGameMode`)))
      (`/Game/Assets/Blueprints/GameManager/GM_ToxBoxInGame.AddCurrentStar` _asgm_tox_box_in_game)
      (`/Game/Assets/Blueprints/GameManager/GM_ToxBoxInGame.AddScore` _asgm_tox_box_in_game 1000)
      (`GameplayStatics.PlaySound2D` "/Game/Assets/Audio/Collectables/GetStar.GetStar" 1.0 (`KismetMathLibrary.RandomFloatInRange` 0.8 1.2) 0.0 null null)
      (`self.K2_DestroyActor`))
    (:`CastFailed`
      (bind _asbp_fake_player (cast `/Game/Assets/Blueprints/FakePlayers/BP_FakePlayer` OtherActor))
      (`/Game/Assets/Blueprints/FakePlayers/BP_FakePlayer.SetAnimWin` _asbp_fake_player)
      (bind _asgm_tox_box_in_game_2 (cast `/Game/Assets/Blueprints/GameManager/GM_ToxBoxInGame` (`GameplayStatics.GetGameMode`)))
      (`/Game/Assets/Blueprints/GameManager/GM_ToxBoxInGame.AddScore` _asgm_tox_box_in_game_2 -250)
      (`self.K2_DestroyActor`))))

(fn `UserConstructionScript`)