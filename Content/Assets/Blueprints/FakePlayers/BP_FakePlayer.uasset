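; BP_FakePlayer is an AI stand-in player that moves in random grid steps until killed.
; SetMoveCase runs CheckSide's downward traces, rejecting gaps, lever platforms and cube players, then rolls a direction index that never reaches Right.
; Tick interpolates location and yaw toward that cell and copies the step count from the camera player's followed actor.
; SetDeath stops movement, gravity and collision, then ragdolls the mesh after a delay.
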(event `SetDeath`
  (bind _capsulecomponent (`self.CapsuleComponent`))
  (if (not (`self.IsDead`))
    (set `self.IsDead` true)
    (set `self.CanMove` false)
    (`PrimitiveComponent.SetEnableGravity` _capsulecomponent false)
    (`PrimitiveComponent.SetCollisionEnabled` _capsulecomponent "NoCollision")
    (`KismetSystemLibrary.K2_SetTimerDelegate` (delegate `SetRagdoll`) 3.0)))

(event `SetRagdoll`
  (`PrimitiveComponent.SetSimulatePhysics` (`self.Mesh`) true))

(event `self.ReceiveTick`
  (params (DeltaSeconds :type "Float (single-precision)"))
  (set `self.Delta Seconds` DeltaSeconds)
  (`self.MoveCaseInterp` (`self.PlayerIsMoving`))
  (`|ExecutionSequence`
    (:`then_0`
      (`self.GetPlayer`)
      (`self.GetStepLocal`))))

(event `SetMoveCase`
  (bind _int (`self.MoveCase`))
  (set `self.PlayerIsMoving` _int))

(fn `CheckSide`
  (returns (Up :type Boolean) (Down :type Boolean) (Left :type Boolean) (Right :type Boolean))
  (locals (LocalUp :type Boolean) (LocalDown :type Boolean) (LocalLeft :type Boolean) (LocalRight :type Boolean))
  (bind (_returnvalue_x _returnvalue_y _returnvalue_z) (`KismetMathLibrary.BreakVector` (`self.K2_GetActorLocation`)))
  (bind (_returnvalue_x_2 _returnvalue_y_2 _returnvalue_z_2) (`KismetMathLibrary.BreakVector` (`self.K2_GetActorLocation`)))
  (bind (_returnvalue_x_3 _returnvalue_y_3 _returnvalue_z_3) (`KismetMathLibrary.BreakVector` (`self.K2_GetActorLocation`)))
  (bind (_returnvalue_x_4 _returnvalue_y_4 _returnvalue_z_4) (`KismetMathLibrary.BreakVector` (`self.K2_GetActorLocation`)))
  (bind (_returnvalue_x_5 _returnvalue_y_5 _returnvalue_z_5) (`KismetMathLibrary.BreakVector` (`self.K2_GetActorLocation`)))
  (bind (_returnvalue_x_6 _returnvalue_y_6 _returnvalue_z_6) (`KismetMathLibrary.BreakVector` (`self.K2_GetActorLocation`)))
  (bind (_returnvalue_x_7 _returnvalue_y_7 _returnvalue_z_7) (`KismetMathLibrary.BreakVector` (`self.K2_GetActorLocation`)))
  (bind (_returnvalue_x_8 _returnvalue_y_8 _returnvalue_z_8) (`KismetMathLibrary.BreakVector` (`self.K2_GetActorLocation`)))
  (`|ExecutionSequence`
    (:`then_0`
      ;[1 1 1] Forward
      (bind (_outhit _returnvalue) (`KismetSystemLibrary.LineTraceSingleForObjects` :`Start` (`KismetMathLibrary.MakeVector` _returnvalue_x_2 _returnvalue_y_2 (+ _returnvalue_z_2 50.0)) :`End` (`KismetMathLibrary.MakeVector` (+ _returnvalue_x_3 100.0) _returnvalue_y_3 (+ _returnvalue_z_3 -100.0)) :`ObjectTypes` (`|MakeArray` "ObjectTypeQuery1" "ObjectTypeQuery2" "ObjectTypeQuery3" :!type "EObjectTypeQuery Enum") :`DrawDebugType` (select `bool` (`self.DebugMode`) :`true` "ForDuration" :!type "EDrawDebugTrace Enum") :`DrawTime` 0.05))
      (if _returnvalue
        (bind (_bblockinghit _binitialoverlap _time _distance _location _impactpoint _normal _impactnormal _physmat _hitactor) (`GameplayStatics.BreakHitResult` _outhit))
        (cast `/Game/Assets/Blueprints/Gameplay/BP_LeverPlatform` _hitactor
          (:`then`
            (set `local.LocalUp` false :!label _label))
          (:`CastFailed`
            (cast `/Game/Assets/Blueprints/Players/BP_CubePlayer` _hitactor
              (:`then`
                (goto _label))
              (:`CastFailed`
                (set `local.LocalUp` true)))))
        (else
          (goto _label))))
    (:`then_1`
      ;[1 1 1] Backward
      (bind (_outhit_2 _returnvalue_2) (`KismetSystemLibrary.LineTraceSingleForObjects` :`Start` (`KismetMathLibrary.MakeVector` _returnvalue_x_4 _returnvalue_y_4 (+ _returnvalue_z_4 50.0)) :`End` (`KismetMathLibrary.MakeVector` (+ _returnvalue_x_5 -100.0) _returnvalue_y_5 (+ _returnvalue_z_5 -100.0)) :`ObjectTypes` (`|MakeArray` "ObjectTypeQuery1" "ObjectTypeQuery2" "ObjectTypeQuery3" :!type "EObjectTypeQuery Enum") :`DrawDebugType` (select `bool` (`self.DebugMode`) :`true` "ForDuration" :!type "EDrawDebugTrace Enum") :`DrawTime` 0.05))
      (if _returnvalue_2
        (bind (_bblockinghit_2 _binitialoverlap_2 _time_2 _distance_2 _location_2 _impactpoint_2 _normal_2 _impactnormal_2 _physmat_2 _hitactor_2) (`GameplayStatics.BreakHitResult` _outhit_2))
        (cast `/Game/Assets/Blueprints/Gameplay/BP_LeverPlatform` _hitactor_2
          (:`then`
            (set `local.LocalDown` false :!label _label_2))
          (:`CastFailed`
            (cast `/Game/Assets/Blueprints/Players/BP_CubePlayer` _hitactor_2
              (:`then`
                (goto _label_2))
              (:`CastFailed`
                (set `local.LocalDown` true)))))
        (else
          (goto _label_2))))
    (:`then_2`
      ;[1 1 1] Left
      (bind (_outhit_3 _returnvalue_3) (`KismetSystemLibrary.LineTraceSingleForObjects` :`Start` (`KismetMathLibrary.MakeVector` _returnvalue_x_6 _returnvalue_y_6 (+ _returnvalue_z_6 50.0)) :`End` (`KismetMathLibrary.MakeVector` _returnvalue_x_7 (+ _returnvalue_y_7 -100.0) (+ _returnvalue_z_7 -100.0)) :`ObjectTypes` (`|MakeArray` "ObjectTypeQuery1" "ObjectTypeQuery2" "ObjectTypeQuery3" :!type "EObjectTypeQuery Enum") :`DrawDebugType` (select `bool` (`self.DebugMode`) :`true` "ForDuration" :!type "EDrawDebugTrace Enum") :`DrawTime` 0.05))
      (if _returnvalue_3
        (bind (_bblockinghit_3 _binitialoverlap_3 _time_3 _distance_3 _location_3 _impactpoint_3 _normal_3 _impactnormal_3 _physmat_3 _hitactor_3) (`GameplayStatics.BreakHitResult` _outhit_3))
        (cast `/Game/Assets/Blueprints/Gameplay/BP_LeverPlatform` _hitactor_3
          (:`then`
            (set `local.LocalLeft` false :!label _label_3))
          (:`CastFailed`
            (cast `/Game/Assets/Blueprints/Players/BP_CubePlayer` _hitactor_3
              (:`then`
                (goto _label_3))
              (:`CastFailed`
                (set `local.LocalLeft` true)))))
        (else
          (goto _label_3))))
    (:`then_3`
      ;[1 1 1] Right
      (bind (_outhit_4 _returnvalue_4) (`KismetSystemLibrary.LineTraceSingleForObjects` :`Start` (`KismetMathLibrary.MakeVector` _returnvalue_x _returnvalue_y (+ _returnvalue_z 50.0)) :`End` (`KismetMathLibrary.MakeVector` _returnvalue_x_8 (+ _returnvalue_y_8 100.0) (+ _returnvalue_z_8 -100.0)) :`ObjectTypes` (`|MakeArray` "ObjectTypeQuery1" "ObjectTypeQuery2" "ObjectTypeQuery3" :!type "EObjectTypeQuery Enum") :`DrawDebugType` (select `bool` (`self.DebugMode`) :`true` "ForDuration" :!type "EDrawDebugTrace Enum") :`DrawTime` 0.05))
      (if _returnvalue_4
        (bind (_bblockinghit_4 _binitialoverlap_4 _time_4 _distance_4 _location_4 _impactpoint_4 _normal_4 _impactnormal_4 _physmat_4 _hitactor_4) (`GameplayStatics.BreakHitResult` _outhit_4))
        (cast `/Game/Assets/Blueprints/Gameplay/BP_LeverPlatform` _hitactor_4
          (:`then`
            (set `local.LocalRight` false :!label _label_4))
          (:`CastFailed`
            (cast `/Game/Assets/Blueprints/Players/BP_CubePlayer` _hitactor_4
              (:`then`
                (goto _label_4))
              (:`CastFailed`
                (set `local.LocalRight` true)))))
        (else
          (goto _label_4))))
    (:`then_4`
      (return (`local.LocalUp`) (`local.LocalDown`) (`local.LocalLeft`) (`local.LocalRight`)))))

(fn `GetPlayer`
  (`/Engine/EditorBlueprintResources/StandardMacros.IsValid` (`self.BP_Player`)
    (:`Is Not Valid`
      (bind _outactors (`GameplayStatics.GetAllActorsOfClass` "/Game/Assets/Blueprints/Players/BP_CameraPlayer.BP_CameraPlayer_C"))
      (for _array_element _outactors
        (set `self.BP_Player` _array_element)
        (break)))))

(fn `GetStepLocal`
  (bind _bp_player (`self.BP_Player`))
  (bind _playerfollow (`/Game/Assets/Blueprints/Players/BP_CameraPlayer.PlayerFollow` _bp_player))
  (`/Engine/EditorBlueprintResources/StandardMacros.IsValid` _bp_player
    (:`Is Valid`
      (`/Engine/EditorBlueprintResources/StandardMacros.IsValid` _playerfollow
        (:`Is Valid`
          (set `self.Local Step Count` (`/Game/Assets/Blueprints/Players/BP_CubePlayer.stepCount` _playerfollow)))))))

(fn `MoveCase`
  (returns (Int :type Integer))
  (locals (RandomInt :type Byte) (ArrayBool :type "Array of Boolean") (SelectedID :type Byte :default 4) (DetectSoloID :type Byte) (DetectSoloBool :type Boolean :default true))
  (if (not (`self.IsDead`))
    (if (`self.CanMove`)
      (set `self.CanMove` false)
      (bind (_up _down _left _right) (`self.CheckSide`))
      (bind _output_get (set `local.ArrayBool` (`|MakeArray` _up _down _left _right)))
      (set `local.RandomInt` (`KismetMathLibrary.Conv_IntToByte` (`KismetMathLibrary.RandomInteger` (- (`KismetArrayLibrary.Array_Length` _output_get) 1))))
      (for (_array_element _array_index) (`local.ArrayBool`)
        (if _array_element
          (if (== _array_index (`local.RandomInt`))
            (set `local.SelectedID` (`KismetMathLibrary.Conv_IntToByte` _array_index))
            (break))))
      (return (`KismetMathLibrary.Conv_ByteToInt` (`local.SelectedID`))))))

(fn `MoveCaseInterp`
  (params (Int :type Integer))
  (bind _returnvalue (`self.K2_GetActorLocation`))
  (bind _returnvalue_2 (`self.K2_GetActorLocation`))
  (bind _returnvalue_3 (`self.K2_GetActorLocation`))
  (bind (_returnvalue_roll _returnvalue_pitch _returnvalue_yaw) (`KismetMathLibrary.BreakRotator` (`self.K2_GetActorRotation`)))
  (bind _returnvalue_4 (`self.K2_GetActorLocation`))
  (bind (_returnvalue_roll_2 _returnvalue_pitch_2 _returnvalue_yaw_2) (`KismetMathLibrary.BreakRotator` (`self.K2_GetActorRotation`)))
  (bind (_returnvalue_roll_3 _returnvalue_pitch_3 _returnvalue_yaw_3) (`KismetMathLibrary.BreakRotator` (`self.K2_GetActorRotation`)))
  (bind (_returnvalue_roll_4 _returnvalue_pitch_4 _returnvalue_yaw_4) (`KismetMathLibrary.BreakRotator` (`self.K2_GetActorRotation`)))
  (bind _vectormovement (`self.VectorMovement`))
  (bind _vectormovement_2 (`self.VectorMovement`))
  (bind _vectormovement_3 (`self.VectorMovement`))
  (bind _vectormovement_4 (`self.VectorMovement`))
  (bind _vectormovement_5 (`self.VectorMovement`))
  (bind (_x _y _z) (`KismetMathLibrary.BreakVector3f` _returnvalue_4))
  (bind (_x_2 _y_2 _z_2) (`KismetMathLibrary.BreakVector3f` _returnvalue))
  (bind (_x_3 _y_3 _z_3) (`KismetMathLibrary.BreakVector3f` _returnvalue))
  (bind (_x_4 _y_4 _z_4) (`KismetMathLibrary.BreakVector3f` _returnvalue_2))
  (bind (_x_5 _y_5 _z_5) (`KismetMathLibrary.BreakVector3f` _returnvalue_2))
  (bind (_x_6 _y_6 _z_6) (`KismetMathLibrary.BreakVector3f` _returnvalue_3))
  (bind (_x_7 _y_7 _z_7) (`KismetMathLibrary.BreakVector3f` _returnvalue_3))
  (bind (_x_8 _y_8 _z_8) (`KismetMathLibrary.BreakVector3f` _returnvalue_4))
  (bind _output (`|GetArrayItem` _vectormovement_5 3))
  (bind _output_2 (`|GetArrayItem` _vectormovement 1))
  (bind _output_3 (`|GetArrayItem` _vectormovement_2 2))
  (bind _output_4 (`|GetArrayItem` _vectormovement_3))
  (bind (_returnvalue_roll_5 _returnvalue_pitch_5 _returnvalue_yaw_5) (`KismetMathLibrary.BreakRotator` (`KismetMathLibrary.FindLookAtRotation` (`self.K2_GetActorLocation`) (`|GetArrayItem` (`self.VectorMovement`) 3))))
  (bind (_returnvalue_roll_6 _returnvalue_pitch_6 _returnvalue_yaw_6) (`KismetMathLibrary.BreakRotator` (`KismetMathLibrary.FindLookAtRotation` (`self.K2_GetActorLocation`) (`|GetArrayItem` (`self.VectorMovement`)))))
  (bind (_returnvalue_roll_7 _returnvalue_pitch_7 _returnvalue_yaw_7) (`KismetMathLibrary.BreakRotator` (`KismetMathLibrary.FindLookAtRotation` (`self.K2_GetActorLocation`) (`|GetArrayItem` (`self.VectorMovement`) 1))))
  (bind (_returnvalue_roll_8 _returnvalue_pitch_8 _returnvalue_yaw_8) (`KismetMathLibrary.BreakRotator` (`KismetMathLibrary.FindLookAtRotation` (`self.K2_GetActorLocation`) (`|GetArrayItem` (`self.VectorMovement`) 2))))
  ;[1 0.08653 0.1962] Logic Preparation
  (if (not (`self.IsDead`))
    (if (!= Int -1)
      (switch `int` (`self.PlayerIsMoving`)
        (:`Default`
          ;[1 0.7599 0.617] Reset
          (set `self.PlayerIsMoving` -1))
        (:`0`
          ;[0.5406 0.04144 1] UP
          (if (!= _output_4 (0.0 0.0 0.0))
            (`self.K2_SetActorLocation` (`KismetMathLibrary.MakeVector` (`KismetMathLibrary.FInterpTo` _x_3 (`KismetMathLibrary.BreakVector3f` _output_4) (`self.Delta Seconds`) 5.0) _y_3 _z_3))
            (`self.K2_SetActorRotation` (`KismetMathLibrary.RInterpTo` (`KismetMathLibrary.MakeRotator` 0.0 0.0 _returnvalue_yaw_2) (`KismetMathLibrary.MakeRotator` 0.0 0.0 _returnvalue_yaw_6) (`self.Delta Seconds`) 5.0))
            (if (== (`self.K2_GetActorLocation`) (`|GetArrayItem` (`self.VectorMovement`)) :`ErrorTolerance` 0.5)
              ;[0.2392 1 0.226] End logic
              (`self.K2_SetActorLocation` (`|GetArrayItem` (`self.VectorMovement`) (`self.PlayerIsMoving`)) :!label _label)
              (set `self.PlayerIsMoving` -1))
            (else
              (`KismetArrayLibrary.Array_Set` _vectormovement_3 0 (`KismetMathLibrary.MakeVector` (+ _x_2 100.0) _y_2 _z_2)))))
        (:`1`
          ;[0.5052 1 0.01042] Down
          (if (!= _output_2 (0.0 0.0 0.0))
            (`self.K2_SetActorLocation` (`KismetMathLibrary.MakeVector` (`KismetMathLibrary.FInterpTo` _x_5 (`KismetMathLibrary.BreakVector3f` _output_2) (`self.Delta Seconds`) 5.0) _y_5 _z_5))
            (`self.K2_SetActorRotation` (`KismetMathLibrary.RInterpTo` (`KismetMathLibrary.MakeRotator` 0.0 0.0 _returnvalue_yaw_3) (`KismetMathLibrary.MakeRotator` 0.0 0.0 _returnvalue_yaw_7) (`self.Delta Seconds`) 5.0))
            (if (== (`self.K2_GetActorLocation`) (`|GetArrayItem` (`self.VectorMovement`) 1) :`ErrorTolerance` 0.5)
              (goto _label))
            (else
              (`KismetArrayLibrary.Array_Set` _vectormovement 1 (`KismetMathLibrary.MakeVector` (- _x_4 100.0) _y_4 _z_4)))))
        (:`2`
          ;[0 1 0.9674] Left
          (if (!= _output_3 (0.0 0.0 0.0))
            (`self.K2_SetActorLocation` (`KismetMathLibrary.MakeVector` _x_7 (`KismetMathLibrary.FInterpTo` _y_7 (`.Y` (`KismetMathLibrary.BreakVector3f` _output_3)) (`self.Delta Seconds`) 5.0) _z_7))
            (`self.K2_SetActorRotation` (`KismetMathLibrary.RInterpTo` (`KismetMathLibrary.MakeRotator` 0.0 0.0 _returnvalue_yaw_4) (`KismetMathLibrary.MakeRotator` 0.0 0.0 _returnvalue_yaw_8) (`self.Delta Seconds`) 5.0))
            (if (== (`self.K2_GetActorLocation`) (`|GetArrayItem` (`self.VectorMovement`) 2) :`ErrorTolerance` 0.5)
              (goto _label))
            (else
              (`KismetArrayLibrary.Array_Set` _vectormovement_2 2 (`KismetMathLibrary.MakeVector` _x_6 (- _y_6 100.0) _z_6)))))
        (:`3`
          ;[1 0.02255 0] Right
          (if (!= _output (0.0 0.0 0.0))
            (`self.K2_SetActorLocation` (`KismetMathLibrary.MakeVector` _x_8 (`KismetMathLibrary.FInterpTo` _y_8 (`.Y` (`KismetMathLibrary.BreakVector3f` _output)) (`self.Delta Seconds`) 5.0) _z_8))
            (`self.K2_SetActorRotation` (`KismetMathLibrary.RInterpTo` (`KismetMathLibrary.MakeRotator` 0.0 0.0 _returnvalue_yaw) (`KismetMathLibrary.MakeRotator` 0.0 0.0 _returnvalue_yaw_5) (`self.Delta Seconds`) 5.0))
            (if (== (`self.K2_GetActorLocation`) (`|GetArrayItem` (`self.VectorMovement`) 3) :`ErrorTolerance` 0.5)
              (goto _label))
            (else
              (`KismetArrayLibrary.Array_Set` _vectormovement_5 3 (`KismetMathLibrary.MakeVector` _x (+ _y 100.0) _z))))))
      (else
        (for (_ _array_index) _vectormovement_4
          (`KismetArrayLibrary.Array_Set` _vectormovement_4 _array_index))))))

(fn `UserConstructionScript`)