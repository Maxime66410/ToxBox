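; In-game manager for a ToxBox level, tracking score, elapsed time, pause and level completion.
; On BeginPlay it gathers fake players, stars and four coin types, creates the InGame UI linked to the camera player, then runs a save-data test overwriting the first level's best score.
; Pickups fill parallel bool arrays; completing all stars or fake players triggers score calculation after a short delay.
; A self-rescheduling one-second timer counts time.
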(event `self.ReceiveBeginPlay`
  (`self.GetInstancedObject`)
  (`self.GetPlayer`)
  (`self.SetupUI`)
  (`self.InitGameData`))

(event `AddScore`
  (params (Int :type Integer))
  (set `self.Score` (+ (`self.Score`) Int))
  (`/Game/Assets/Blueprints/Interface/HUD/UI_InGame.SetScoreAddPointAnimation` (`self.InGame`) (`KismetTextLibrary.Conv_StringToText` (`KismetStringLibrary.Concat_StrStr` "+" (`KismetStringLibrary.Conv_IntToString` Int)))))

(event `IsPauseLogic?`
  (params (`IsPause?` :type Boolean))
  (bind _output_get (set `self.IsPause?` `IsPause?`))
  (if (not _output_get)
    (`self.TimerSystem`)))

(event `StartDelayCheckIfFinish`
  (params (`IsStar?` :type Boolean))
  (`KismetSystemLibrary.Delay` 0.5)
  (`self.GetIsFinish` `IsStar?`))

(event `StartGame`
  (set `self.IsStart?` true)
  (`self.TimerSystem`))

(event `TimerSystem`
  (`/Engine/EditorBlueprintResources/StandardMacros.IncrementFloat` (`self.Time`)
    (:`  `
      (if (not (`self.IsFinish?`))
        (if (not (`self.IsPause?`))
          (`KismetSystemLibrary.K2_SetTimerDelegate` (delegate `TimerSystem`) 1.0))))))

(event `SetIsFinish`
  (set `self.IsFinish?` true)
  (`/Game/Assets/Blueprints/Interface/HUD/UI_InGame.CalculateScore` (`self.InGame`)))

(fn `AddCurrentCoins`
  (bind _boolcoins (`self.BoolCoins`))
  (for (_array_element _array_index) _boolcoins
    (if (not _array_element)
      (`KismetArrayLibrary.Array_Set` _boolcoins _array_index true)
      (break))))

(fn `AddCurrentFakePlr`
  (bind _boolfakeplr (`self.BoolFakePlr`))
  (for (_array_element _array_index) _boolfakeplr
    (if (not _array_element)
      (`KismetArrayLibrary.Array_Set` _boolfakeplr _array_index true)
      (break)))
  (`self.StartDelayCheckIfFinish` false))

(fn `AddCurrentStar`
  (bind _boolstar (`self.BoolStar`))
  (for (_array_element _array_index) _boolstar
    (if (not _array_element)
      (`KismetArrayLibrary.Array_Set` _boolstar _array_index true)
      (break)))
  (`self.StartDelayCheckIfFinish` true))

(fn `GetCurrentCoins`
  (returns (TextOut :type String))
  (locals (NbrOut :type Integer))
  (for _array_element (`self.BoolCoins`)
    (if _array_element
      (`/Engine/EditorBlueprintResources/StandardMacros.IncrementInt` (`local.NbrOut`))))
  (return (`KismetStringLibrary.Conv_IntToString` (`local.NbrOut`))))

(fn `GetCurrentFakePlr`
  (returns (TextOut :type String))
  (locals (NbrGet :type Integer))
  (for _array_element (`self.BoolFakePlr`)
    (if _array_element
      (`/Engine/EditorBlueprintResources/StandardMacros.IncrementInt` (`local.NbrGet`))))
  (return (`KismetStringLibrary.Conv_IntToString` (`local.NbrGet`))))

(fn `GetCurrentStar`
  (returns (TextOut :type String))
  (locals (NbrOut :type Integer :default 0))
  (for _array_element (`self.BoolStar`)
    (if _array_element
      (`/Engine/EditorBlueprintResources/StandardMacros.IncrementInt` (`local.NbrOut`))))
  (return (`KismetStringLibrary.Conv_IntToString` (`local.NbrOut`))))

(fn `GetInstancedObject`
  ;[1 0.1072 0.2169] Get All Fake Plr
  (bind _outactors (`GameplayStatics.GetAllActorsOfClass` "/Game/Assets/Blueprints/FakePlayers/BP_FakePlayer.BP_FakePlayer_C"))
  (for _array_element _outactors
    (`KismetArrayLibrary.Array_Add` (`self.StockFakePlr`) _array_element)
    (`KismetArrayLibrary.Array_Add` (`self.BoolFakePlr`)))
  (set `self.NbrFakePlr` (`KismetArrayLibrary.Array_Length` (`self.StockFakePlr`)))
  ;[1 0.8422 0.1435] Get All Stars
  (bind _outactors_2 (`GameplayStatics.GetAllActorsOfClass` "/Game/Assets/Blueprints/Collectables/BP_StarGold.BP_StarGold_C"))
  (for _array_element_2 _outactors_2
    (`KismetArrayLibrary.Array_Add` (`self.StockStar`) _array_element_2)
    (`KismetArrayLibrary.Array_Add` (`self.BoolStar`)))
  (set `self.NbrStar` (`KismetArrayLibrary.Array_Length` (`self.StockStar`)))
  ;[1 0.04501 0.266] Get All Coins
  ;;[1 0.8822 0.1622] Get Basic Coins
  (bind _outactors_3 (`GameplayStatics.GetAllActorsOfClass` "/Game/Assets/Blueprints/Collectables/BP_Coins.BP_Coins_C"))
  (for _array_element_3 _outactors_3
    (`KismetArrayLibrary.Array_Add` (`self.StockCoins`) _array_element_3)
    (`KismetArrayLibrary.Array_Add` (`self.BoolCoins`)))
  ;;[0.3236 0.8901 1] Get Blue Coins
  (bind _outactors_4 (`GameplayStatics.GetAllActorsOfClass` "/Game/Assets/Blueprints/Collectables/BP_CoinsBlue.BP_CoinsBlue_C"))
  (for _array_element_4 _outactors_4
    (`KismetArrayLibrary.Array_Add` (`self.StockCoins`) _array_element_4)
    (`KismetArrayLibrary.Array_Add` (`self.BoolCoins`)))
  ;;;[0.1875 1 0.1146] Get Green Coins
  (bind _outactors_5 (`GameplayStatics.GetAllActorsOfClass` "/Game/Assets/Blueprints/Collectables/BP_CoinsGreen.BP_CoinsGreen_C"))
  (for _array_element_5 _outactors_5
    (`KismetArrayLibrary.Array_Add` (`self.StockCoins`) _array_element_5)
    (`KismetArrayLibrary.Array_Add` (`self.BoolCoins`)))
  ;;[0.6254 0.2708 1] Get Purple Coins
  (bind _outactors_6 (`GameplayStatics.GetAllActorsOfClass` "/Game/Assets/Blueprints/Collectables/BP_CoinsPurple.BP_CoinsPurple_C"))
  (for _array_element_6 _outactors_6
    (`KismetArrayLibrary.Array_Add` (`self.StockCoins`) _array_element_6)
    (`KismetArrayLibrary.Array_Add` (`self.BoolCoins`)))
  (set `self.NbrCoins` (`KismetArrayLibrary.Array_Length` (`self.StockCoins`))))

(fn `GetIsFinish`
  (params (`IsStar?` :type Boolean))
  (locals (`IsFinish?` :type Integer))
  (if `IsStar?`
    (for _array_element (`self.BoolStar`)
      (if _array_element
        (`/Engine/EditorBlueprintResources/StandardMacros.IncrementInt` (`local.IsFinish?`))
        (else
          (break))))
    (if (== (`local.IsFinish?`) (`self.NbrStar`))
      (`self.SetIsFinish`))
    (else
      (for _array_element_2 (`self.BoolFakePlr`)
        (if _array_element_2
          (`/Engine/EditorBlueprintResources/StandardMacros.IncrementInt` (`local.IsFinish?`))
          (else
            (break))))
      (if (== (`local.IsFinish?`) (`self.NbrFakePlr`))
        (`self.SetIsFinish`)))))

(fn `GetPlayer`
  (bind _outactors (`GameplayStatics.GetAllActorsOfClass` "/Game/Assets/Blueprints/Players/BP_CameraPlayer.BP_CameraPlayer_C"))
  (for _array_element _outactors
    (set `self.Player` _array_element)
    (break)))

(fn `InitGameData`
  (bind _datagame (`self.DataGame`))
  (bind _output (`|GetArrayItem` (`/Game/Assets/Data/BPAS_ListLevelData.ListLevel` _datagame)))
  (`/Game/Assets/Data/BPAS_ListLevelData.LoadData` _datagame)
  (`KismetSystemLibrary.PrintString` (`/Game/Assets/Data/BPAS_LevelGame.NameLevel` _output))
  (`KismetSystemLibrary.PrintString` (`KismetStringLibrary.Conv_IntToString` (`/Game/Assets/Data/BPAS_LevelGame.BestScore` _output)))
  (set `/Game/Assets/Data/BPAS_LevelGame.BestScore` 5 _output)
  (`/Game/Assets/Data/BPAS_ListLevelData.SaveData` _datagame))

(fn `SetupUI`
  (bind _returnvalue (`GameplayStatics.GetPlayerController` 0))
  (bind _player (`self.Player`))
  (bind _ingame (`self.InGame`))
  (bind _returnvalue_2 (`|CreateWidget` "/Game/Assets/Blueprints/Interface/HUD/UI_InGame.UI_InGame_C"))
  (bind _output_get (set `self.InGame` _returnvalue_2))
  (`UserWidget.AddToViewport` _output_get 0)
  (`/Engine/EditorBlueprintResources/StandardMacros.IsValid` _player
    (:`Is Valid`
      (set `/Game/Assets/Blueprints/Players/BP_CameraPlayer.UI_InGame` _ingame _player)
      (set `/Game/Assets/Blueprints/Interface/HUD/UI_InGame.GameManager` self _ingame)
      (`WidgetBlueprintLibrary.SetInputMode_UIOnlyEx` _returnvalue (`self.InGame`) "DoNotLock" true)
      (set `PlayerController.bShowMouseCursor` true _returnvalue))))

(fn `UserConstructionScript`)