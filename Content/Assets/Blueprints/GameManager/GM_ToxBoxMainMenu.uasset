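; Main menu game manager for ToxBox that initializes level progress save data and shows the menu on begin play.
; LoadData reads the ToxBoxData slot into a cached level list, or creates a new SA_DataGame if the cast fails.
; SaveData writes that list back to the slot, and startup runs it right after loading.
; SetupMenu then creates UI_MainMenu, hands it a reference to this manager and adds it to the viewport.
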(event `self.ReceiveBeginPlay`
  (`self.InitGameData`)
  (`self.SetupMenu`))

(event `LoadData`
  ;[1 0.8587 0] LoadData Game
  (bind _returnvalue (`GameplayStatics.LoadGameFromSlot` "ToxBoxData"))
  (bind _assa_data_game (cast `/Game/Assets/Data/SA_DataGame` _returnvalue)
    (:`then`
      (bind _output_get (set `self.As SA Data Game` _assa_data_game))
      (set `self.ListDataGame` (`/Game/Assets/Data/SA_DataGame.ListLevel` _output_get)))
    (:`CastFailed`
      (bind _returnvalue_2 (`GameplayStatics.CreateSaveGameObject` "/Game/Assets/Data/SA_DataGame.SA_DataGame_C"))
      (set `self.As SA Data Game` _returnvalue_2))))

(event `SaveData`
  (bind _listdatagame_list (break `/Game/Assets/Data/ST_ListLevel` (`self.ListDataGame`)))
  ;[1 0.1855 0.1557] Save Data
  (`/Engine/EditorBlueprintResources/StandardMacros.IsValid` (`self.As SA Data Game`)
    (:`Is Valid`
      (setmembers `/Game/Assets/Data/ST_ListLevel` :`StructRef` (`/Game/Assets/Data/SA_DataGame.ListLevel` (`self.As SA Data Game`)) :`List` _listdatagame_list)
      (bind _returnvalue (`GameplayStatics.SaveGameToSlot` (`self.As SA Data Game`) "ToxBoxData"))
      (if _returnvalue
        _))
    (:`Is Not Valid`
      (`self.LoadData`))))

(fn `InitGameData`
  (`self.LoadData`)
  (`self.SaveData`))

(fn `SetupMenu`
  (bind _returnvalue (`|CreateWidget` "/Game/Assets/Blueprints/Interface/MainMenu/UI_MainMenu.UI_MainMenu_C" (`GameplayStatics.GetPlayerController` 0)))
  (bind _output_get (set `self.UI_MainMenu` _returnvalue))
  (set `/Game/Assets/Blueprints/Interface/MainMenu/UI_MainMenu.GM` self _output_get)
  (`UserWidget.AddToViewport` _output_get 0))

(fn `UserConstructionScript`)