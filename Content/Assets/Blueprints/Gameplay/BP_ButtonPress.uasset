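; BP_ButtonPress is a one-shot trigger button that opens a linked target when the cube player touches it.
; A box overlap from BP_CubePlayer sets IsPressed, then calls Open on Target through the BPI_PressButtonENT interface.
; It then swaps the button material and adds score through GM_ToxBoxInGame.
; The material and score steps run only if Target implements the interface, though the button still counts as pressed.
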(event `self.Box.OnComponentBeginOverlap`
  (params (OverlappedComponent :type "PrimitiveComponent Object Reference") (OtherActor :type "Actor Object Reference") (OtherComp :type "PrimitiveComponent Object Reference") (OtherBodyIndex :type Integer) (bFromSweep :type Boolean) (SweepResult :type "HitResult Structure (by ref)"))
  (cast `/Game/Assets/Blueprints/Players/BP_CubePlayer` OtherActor)
  (if (not (`self.IsPressed`))
    (set `self.IsPressed` true)
    (bind _asbpi_press_button_ent (cast `/Game/Assets/Blueprints/Interface/Platform/BPI_PressButtonENT` (`self.Target`)))
    (`/Game/Assets/Blueprints/Interface/Platform/BPI_PressButtonENT.Open` _asbpi_press_button_ent)
    (`PrimitiveComponent.SetMaterial` (`self.Button`) 0 (`self.Material`))
    (bind _asgm_tox_box_in_game (cast `/Game/Assets/Blueprints/GameManager/GM_ToxBoxInGame` (`GameplayStatics.GetGameMode`)))
    (`/Game/Assets/Blueprints/GameManager/GM_ToxBoxInGame.AddScore` _asgm_tox_box_in_game 50)))

(fn `UserConstructionScript`)