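; BP_GeneratorBomb is a rotatable spawner actor that keeps generating BP_FakePlayer actors at its SpawnPoint.
; A timer starts the first spawn after a delay from BeginPlay, and each spawn re-arms a shorter timer, repeating indefinitely.
; The Open event adds a quarter turn to the target yaw, which Tick smoothly approaches with RInterpTo.
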(event `self.ReceiveBeginPlay`
  (set `self.NewRotator` (`self.K2_GetActorRotation`))
  (`KismetSystemLibrary.K2_SetTimerDelegate` (delegate `SpawnActor`) 5.0))

(event `SpawnActor`
  (`|SpawnActorFromClass` "/Game/Assets/Blueprints/FakePlayers/BP_FakePlayer.BP_FakePlayer_C" (`SceneComponent.K2_GetComponentToWorld` (`self.SpawnPoint`)) "AlwaysSpawn" "OverrideRootScale" null null)
  (`KismetSystemLibrary.K2_SetTimerDelegate` (delegate `SpawnActor`) 3.0))

(event `/Game/Assets/Blueprints/Interface/Platform/BPI_PressButtonENT.Open`
  ;[1 0.7427 0.2809] Change Rotate
  (set `self.NewRotator` (`KismetMathLibrary.MakeRotator` (.roll (`self.NewRotator`)) (.pitch (`self.NewRotator`)) (+ (.yaw (`self.NewRotator`)) 90.0))))

(event `self.ReceiveTick`
  (params (DeltaSeconds :type "Float (single-precision)"))
  ;[0.333 0.4293 1] Update Rotate
  (set `self.Delta Seconds` DeltaSeconds)
  (`self.K2_SetActorRotation` (`KismetMathLibrary.RInterpTo` (`self.K2_GetActorRotation`) (`self.NewRotator`) (`self.Delta Seconds`) 3.0)))

(fn `UserConstructionScript`)