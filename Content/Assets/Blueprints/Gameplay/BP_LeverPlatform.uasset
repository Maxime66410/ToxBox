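; Lever platform Blueprint whose pivot rotates gradually once the platform is opened.
; The Open event sets a one-way IsOpen flag, with no logic here to close it again.
; While the flag is set, Tick uses FInterpTo to ease PlatformPivot's relative roll toward the default zero target, leaving pitch and yaw unchanged.
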(event `self.ReceiveTick`
  (params (DeltaSeconds :type "Float (single-precision)"))
  (bind _platformpivot (`self.PlatformPivot`))
  (bind (_relativerotation_roll _relativerotation_pitch _relativerotation_yaw) (`KismetMathLibrary.BreakRotator` (`SceneComponent.RelativeRotation` _platformpivot)))
  (set `self.Delta Seconds` DeltaSeconds)
  (if (`self.IsOpen`)
    (`SceneComponent.K2_SetRelativeRotation` _platformpivot (`KismetMathLibrary.MakeRotator` (`KismetMathLibrary.FInterpTo` _relativerotation_roll 0.0 (`self.Delta Seconds`) 1.0) _relativerotation_pitch _relativerotation_yaw) false false)))

(event `/Game/Assets/Blueprints/Interface/Platform/BPI_PressButtonENT.Open`
  (if (not (`self.IsOpen`))
    (set `self.IsOpen` true)))

(fn `UserConstructionScript`)