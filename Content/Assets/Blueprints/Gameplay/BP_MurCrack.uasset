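; BP_MurCrack is a breakable wall that shatters into Chaos Geometry Collection debris.
; The first HitWall call removes the Box, disables clustering and enables physics, then schedules a material swap and later actor destruction.
; FadeMat applies dynamic fade material instances to two slots.
; A self-rescheduling FadeStart timer steps Alpha down, though nothing in this graph starts it.
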(event `HitWall`
  (bind _murcrack_geometrycollection (`self.MurCrack_GeometryCollection`))
  ;[1 0.1656 0.2054] On Hit
  (`/Engine/EditorBlueprintResources/StandardMacros.DoOnce` false
    (:`Completed`
      (`ActorComponent.K2_DestroyComponent` (`self.Box`))
      (set `GeometryCollectionComponent.EnableClustering` false _murcrack_geometrycollection)
      (`PrimitiveComponent.SetSimulatePhysics` _murcrack_geometrycollection true)
      (`KismetSystemLibrary.K2_SetTimerDelegate` (delegate `DestroyObject`) 20.0)
      (`KismetSystemLibrary.K2_SetTimerDelegate` (delegate `FadeMat`) 5.0))))

(event `DestroyObject`
  ;[0.34 1 0.1864] Destroy Actor
  (`self.K2_DestroyActor`))

(event `FadeMat`
  (bind _murcrack_geometrycollection (`self.MurCrack_GeometryCollection`))
  ;[0.9798 1 0.02567] Init Fade
  (`PrimitiveComponent.CreateDynamicMaterialInstance` _murcrack_geometrycollection 0 "/Game/Assets/Model/MurCrack/M_MurCrack_Inst.M_MurCrack_Inst" "None")
  (`PrimitiveComponent.CreateDynamicMaterialInstance` _murcrack_geometrycollection 1 "/Game/Assets/Model/MurCrack/M_MurCrack_Inst.M_MurCrack_Inst" "None"))

(event `FadeStart`
  (bind _opacity (`self.Opacity`))
  ;[0.3901 1 0.9202] Fade Logic
  (if (> _opacity 0.0)
    (set `self.Opacity` (- _opacity 0.05))
    (`MeshComponent.SetScalarParameterValueOnMaterials` (`self.MurCrack_GeometryCollection`) "Alpha" (`self.Opacity`))
    (`KismetSystemLibrary.K2_SetTimerDelegate` (delegate `FadeStart`) 0.1)))

(fn `UserConstructionScript`)