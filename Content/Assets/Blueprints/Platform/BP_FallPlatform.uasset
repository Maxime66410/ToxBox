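; BP_FallPlatform is a platform that drops after a countdown once BP_CubePlayer overlaps its trigger.
; The first overlap shows a UI3D_FallTime widget, which holds a reference back to the platform, and starts a self-rescheduling one-second timer that decrements CurrentCount.
; At zero it destroys the trigger, hides the widget and enables physics on the mesh, then destroys the actor five seconds later.
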(event `self.ReceiveBeginPlay`
  (bind _ui_widget (`self.UI_Widget`))
  (bind _asui3d_fall_time (cast `/Game/Assets/Blueprints/Interface/3D/UI3D_FallTime` (`WidgetComponent.GetWidget` (`self.Widget`))))
  (set `self.UI_Widget` _asui3d_fall_time)
  (set `/Game/Assets/Blueprints/Interface/3D/UI3D_FallTime.BP_FallPlatForm` self _ui_widget)
  (set `Widget.Visibility` "Hidden" _ui_widget))

(event `self.Trigger.OnComponentBeginOverlap`
  (params (OverlappedComponent :type "PrimitiveComponent Object Reference") (OtherActor :type "Actor Object Reference") (OtherComp :type "PrimitiveComponent Object Reference") (OtherBodyIndex :type Integer) (bFromSweep :type Boolean) (SweepResult :type "HitResult Structure (by ref)"))
  (cast `/Game/Assets/Blueprints/Players/BP_CubePlayer` OtherActor)
  (if (not (`self.DestroyPlatform`))
    (set `self.DestroyPlatform` true)
    (`self.Delay`)
    (set `Widget.Visibility` "Visible" (`self.UI_Widget`))))

(event `Delay`
  (if (< 0 (`self.CurrentCount`))
    (`/Engine/EditorBlueprintResources/StandardMacros.DecrementInt` (`self.CurrentCount`)
      (:`  `
        (`KismetSystemLibrary.K2_SetTimerDelegate` (delegate `Delay`) 1.0)))
    (else
      (`self.DestroyPlatformEvent`))))

(event `DestroyPlatformEvent`
  (`ActorComponent.K2_DestroyComponent` (`self.Trigger`))
  (`PrimitiveComponent.SetSimulatePhysics` (`self.StaticMesh`) true)
  (`KismetSystemLibrary.K2_SetTimerDelegate` (delegate `RealDestroy`) 5.0)
  (set `Widget.Visibility` "Hidden" (`self.UI_Widget`)))

(event `RealDestroy`
  (`self.K2_DestroyActor`))

(fn `UserConstructionScript`)