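; Player camera pawn that follows the BP_CubePlayer, applies pitch-limited look input and relays directional input to the cube.
; BeginPlay finds the cube, or spawns one at a PlayerStart, and registers itself as its controller reference.
; Move presses pass pause, fall and per-side wall checks before calling StartMoving on the cube.
; Tick snaps the camera to the cube or spectator target, while Escape toggles game-mode pause and cursor.
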(event `InputAction|DebugMode`
  (params (Key :type "Key Structure"))
  (:`Pressed`
    (`/Engine/EditorBlueprintResources/StandardMacros.FlipFlop`
      (:`A`
        (set `self.DebugMode` true))
      (:`B`
        (set `self.DebugMode` false)))
    (set `/Game/Assets/Blueprints/Players/BP_CubePlayer.DebugMode` (`self.DebugMode`) (`self.PlayerFollow`))))

(event `InputAction|Left`
  (params (Key :type "Key Structure"))
  (:`Pressed`
    (`self.CanMoveMacro`
      (:`true`
        (`self.ReturnMoveByWallCheck` "NewEnumerator0"
          (:`false`
            (`/Game/Assets/Blueprints/Players/BP_CubePlayer.StartMoving` (`self.PlayerFollow`) -1 0)))))))

(event `InputAxis|LookUp`
  (params (AxisValue :type "Float (single-precision)"))
  (`self.AddControllerPitchInput` AxisValue))

(event `InputAxis|LookRight`
  (params (AxisValue :type "Float (single-precision)"))
  (`self.AddControllerYawInput` AxisValue))

(event `InputAction|Right`
  (params (Key :type "Key Structure"))
  (:`Pressed`
    (`self.CanMoveMacro`
      (:`true`
        (`self.ReturnMoveByWallCheck` "NewEnumerator1"
          (:`false`
            (`/Game/Assets/Blueprints/Players/BP_CubePlayer.StartMoving` (`self.PlayerFollow`) 1 0)))))))

(event `Key|Escape`
  (params (Key :type "Key Structure"))
  (bind _returnvalue (`GameplayStatics.GetPlayerController` 0))
  ;[0.7278 1 0.09495] PauseLogic
  (:`Pressed`
    (`/Engine/EditorBlueprintResources/StandardMacros.DoOnce` false :!label _label
      (:`Completed`
        (bind _asgm_tox_box_in_game (cast `/Game/Assets/Blueprints/GameManager/GM_ToxBoxInGame` (`GameplayStatics.GetGameMode`)))
        (bind _ispause_ (`/Game/Assets/Blueprints/GameManager/GM_ToxBoxInGame.GetIsPauseLogic?` _asgm_tox_box_in_game))
        (if _ispause_
          (`/Game/Assets/Blueprints/GameManager/GM_ToxBoxInGame.IsPauseLogic?` _asgm_tox_box_in_game false)
          (set `PlayerController.bShowMouseCursor` false _returnvalue)
          (else
            (`/Game/Assets/Blueprints/GameManager/GM_ToxBoxInGame.IsPauseLogic?` _asgm_tox_box_in_game true)
            (set `PlayerController.bShowMouseCursor` true _returnvalue))))))
  (:`Released`
    (goto _label :!via `Reset`)))

(event `Key|Gamepad_Special_Right`
  (params (Key :type "Key Structure"))
  ;[0.7278 1 0.09495] PauseLogic
  (:`Pressed`
    (goto _label))
  (:`Released`
    (goto _label :!via `Reset`)))

(event `self.ReceiveBeginPlay`
  (`self.GetPlayer`)
  (`self.LimitCamera`))

(event `InputAction|Forward`
  (params (Key :type "Key Structure"))
  (:`Pressed`
    (`self.CanMoveMacro`
      (:`true`
        (`self.ReturnMoveByWallCheck` "NewEnumerator2"
          (:`false`
            (`/Game/Assets/Blueprints/Players/BP_CubePlayer.StartMoving` (`self.PlayerFollow`) 0 1)))))))

(event `self.ReceiveTick`
  (params (DeltaSeconds :type "Float (single-precision)"))
  (set `self.Delta Seconds` DeltaSeconds)
  (`|ExecutionSequence`
    (:`then_0`
      (`self.MoveCameraToPlayer`))))

(event `InputAction|Backward`
  (params (Key :type "Key Structure"))
  (:`Pressed`
    (`self.CanMoveMacro`
      (:`true`
        (`self.ReturnMoveByWallCheck` "NewEnumerator3"
          (:`false`
            (`/Game/Assets/Blueprints/Players/BP_CubePlayer.StartMoving` (`self.PlayerFollow`) 0 -1)))))))

(event `SetItemToFocus`
  (params (BoolSpectator :type Boolean) (ActorToFollow :type "Actor Object Reference"))
  ;[0.3177 0.2124 0.08546] Set Spectator Mode
  (set `self.ActorToFollow` ActorToFollow)
  (set `self.BoolSpectator` BoolSpectator))

(fn `AddCoins`
  (params (B :type Integer))
  (set `self.Coins` (+ (`self.Coins`) B)))

(fn `AICanMove`
  (bind _outactors (`GameplayStatics.GetAllActorsOfClass` "/Game/Assets/Blueprints/FakePlayers/BP_FakePlayer.BP_FakePlayer_C"))
  (for _array_element _outactors
    (set `/Game/Assets/Blueprints/FakePlayers/BP_FakePlayer.CanMove` true _array_element)
    (`/Game/Assets/Blueprints/FakePlayers/BP_FakePlayer.SetMoveCase` _array_element)))

(fn `GetPlayer`
  (bind _playerfollow (`self.PlayerFollow`))
  (bind _playerfollow_2 (`self.PlayerFollow`))
  (bind (_returnvalue_x _returnvalue_y) (`KismetMathLibrary.BreakVector` (`self.K2_GetActorLocation` _playerfollow_2)))
  (bind (_returnvalue_x_2 _returnvalue_y_2) (`KismetMathLibrary.BreakVector` (`self.K2_GetActorLocation` _playerfollow)))
  (`/Engine/EditorBlueprintResources/StandardMacros.IsValid` (`self.PlayerFollow`)
    (:`Is Not Valid`
      (bind _outactors (`GameplayStatics.GetAllActorsOfClass` "/Game/Assets/Blueprints/Players/BP_CubePlayer.BP_CubePlayer_C"))
      (if (!= (`KismetArrayLibrary.Array_Length` _outactors) 0)
        ;[1 1 1] Get Player
        (for _array_element _outactors
          (set `self.PlayerFollow` _array_element)
          (break))
        (set `self.PlayerLocationX` _returnvalue_x)
        (set `self.PlayerLocationY` _returnvalue_y)
        (set `/Game/Assets/Blueprints/Players/BP_CubePlayer.ControllerREF` self _playerfollow_2)
        (else
          ;[1 1 1] Create Player if don't exist
          (bind _outactors_2 (`GameplayStatics.GetAllActorsOfClass` "/Script/Engine.PlayerStart"))
          (for _array_element_2 _outactors_2
            (bind (_returnvalue_location _returnvalue_rotation) (`KismetMathLibrary.BreakTransform` (`self.GetTransform` _array_element_2)))
            (bind _returnvalue (`|SpawnActorFromClass` "/Game/Assets/Blueprints/Players/BP_CubePlayer.BP_CubePlayer_C" (`KismetMathLibrary.MakeTransform` _returnvalue_location _returnvalue_rotation) "AdjustIfPossibleButAlwaysSpawn" "OverrideRootScale" null null))
            (set `self.PlayerFollow` _returnvalue)
            (break))
          (set `self.PlayerLocationX` _returnvalue_x_2)
          (set `self.PlayerLocationY` _returnvalue_y_2)
          (set `/Game/Assets/Blueprints/Players/BP_CubePlayer.ControllerREF` self _playerfollow))))))

(fn `LimitCamera`
  (bind _returnvalue (`GameplayStatics.GetPlayerCameraManager` 0))
  (set `PlayerCameraManager.ViewPitchMax` 50.0 _returnvalue)
  (set `PlayerCameraManager.ViewPitchMin` -50.0 _returnvalue))

(fn `MoveCameraToPlayer`
  (bind _playerfollow (`self.PlayerFollow`))
  (bind _actortofollow (`self.ActorToFollow`))
  (`/Engine/EditorBlueprintResources/StandardMacros.IsValid` _playerfollow
    (:`Is Valid`
      (if (not (`self.BoolSpectator`))
        (`self.K2_SetActorLocation` (`self.K2_GetActorLocation` _playerfollow))
        (else
          ;[0.1667 0.1667 0.1667] Spectator Mode Camera
          (`/Engine/EditorBlueprintResources/StandardMacros.IsValid` _actortofollow :!label _label
            (:`Is Valid`
              (`self.K2_SetActorLocation` (`self.K2_GetActorLocation` _actortofollow)))))))
    (:`Is Not Valid`
      (goto _label))))

(fn `UserConstructionScript`)