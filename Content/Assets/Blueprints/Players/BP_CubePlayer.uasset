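; Player cube that rolls in quarter turns along X or Y and falls when no surface lies beneath it.
; StartMoving runs a looping MoveTween timer that rotates location and orientation around an edge pivot in steps, ignoring new moves until done.
; Each tick, line traces set four directional Block flags, which are not read here, and check for ground.
; Losing ground enables mesh physics and schedules a one-time velocity reset.
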(event `self.ReceiveTick`
  (params (DeltaSeconds :type "Float (single-precision)"))
  (set `self.Delta Seconds` DeltaSeconds)
  (`|ExecutionSequence`
    (:`then_0`
      (`self.IsAlwaysSurface`))
    (:`then_1`
      (`self.CheckSideCube`))
    (:`then_2`
      (`self.CheckSurfaceBool`)
      (if (`self.IsFall`)
        (`/Engine/EditorBlueprintResources/StandardMacros.DoOnce` false
          (:`Completed`
            (`KismetSystemLibrary.K2_SetTimer` null "ResetVelocity" 0.035)))))))

(fn `CheckSideCube`
  (bind (_returnvalue_x _returnvalue_y _returnvalue_z) (`KismetMathLibrary.BreakVector` (`self.K2_GetActorLocation`)))
  (bind (_returnvalue_x_2 _returnvalue_y_2 _returnvalue_z_2) (`KismetMathLibrary.BreakVector` (`self.K2_GetActorLocation`)))
  (bind (_returnvalue_x_3 _returnvalue_y_3 _returnvalue_z_3) (`KismetMathLibrary.BreakVector` (`self.K2_GetActorLocation`)))
  (bind (_returnvalue_x_4 _returnvalue_y_4 _returnvalue_z_4) (`KismetMathLibrary.BreakVector` (`self.K2_GetActorLocation`)))
  (bind (_returnvalue_x_5 _returnvalue_y_5 _returnvalue_z_5) (`KismetMathLibrary.BreakVector` (`self.K2_GetActorLocation`)))
  (bind (_returnvalue_x_6 _returnvalue_y_6 _returnvalue_z_6) (`KismetMathLibrary.BreakVector` (`self.K2_GetActorLocation`)))
  (bind (_returnvalue_x_7 _returnvalue_y_7 _returnvalue_z_7) (`KismetMathLibrary.BreakVector` (`self.K2_GetActorLocation`)))
  (bind (_returnvalue_x_8 _returnvalue_y_8 _returnvalue_z_8) (`KismetMathLibrary.BreakVector` (`self.K2_GetActorLocation`)))
  (if (not (`self.IsFall`))
    (`|ExecutionSequence`
      (:`then_0`
        ;[1 1 1] Forward
        (bind (_outhit _returnvalue) (`KismetSystemLibrary.LineTraceSingleForObjects` :`Start` (`KismetMathLibrary.MakeVector` _returnvalue_x_2 _returnvalue_y_2 (+ _returnvalue_z_2 50.0)) :`End` (`KismetMathLibrary.MakeVector` (+ _returnvalue_x_3 100.0) _returnvalue_y_3 (+ _returnvalue_z_3 0.0)) :`ObjectTypes` (`|MakeArray` "ObjectTypeQuery1" "ObjectTypeQuery2" :!type "EObjectTypeQuery Enum") :`DrawDebugType` (select `bool` (`self.DebugMode`) :`true` "ForDuration" :!type "EDrawDebugTrace Enum") :`DrawTime` 0.05))
        (if _returnvalue
          (set `self.BlockForward` true)
          (else
            (set `self.BlockForward` false))))
      (:`then_1`
        ;[1 1 1] Backward
        (bind (_outhit_2 _returnvalue_2) (`KismetSystemLibrary.LineTraceSingleForObjects` :`Start` (`KismetMathLibrary.MakeVector` _returnvalue_x_4 _returnvalue_y_4 (+ _returnvalue_z_4 50.0)) :`End` (`KismetMathLibrary.MakeVector` (+ _returnvalue_x_5 -100.0) _returnvalue_y_5 (+ _returnvalue_z_5 0.0)) :`ObjectTypes` (`|MakeArray` "ObjectTypeQuery1" "ObjectTypeQuery2" :!type "EObjectTypeQuery Enum") :`DrawDebugType` (select `bool` (`self.DebugMode`) :`true` "ForDuration" :!type "EDrawDebugTrace Enum") :`DrawTime` 0.05))
        (if _returnvalue_2
          (set `self.BlockBackward` true)
          (else
            (set `self.BlockBackward` false))))
      (:`then_2`
        ;[1 1 1] Left
        (bind (_outhit_3 _returnvalue_3) (`KismetSystemLibrary.LineTraceSingleForObjects` :`Start` (`KismetMathLibrary.MakeVector` _returnvalue_x_6 _returnvalue_y_6 (+ _returnvalue_z_6 50.0)) :`End` (`KismetMathLibrary.MakeVector` _returnvalue_x_7 (+ _returnvalue_y_7 -100.0) (+ _returnvalue_z_7 0.0)) :`ObjectTypes` (`|MakeArray` "ObjectTypeQuery1" "ObjectTypeQuery2" :!type "EObjectTypeQuery Enum") :`DrawDebugType` (select `bool` (`self.DebugMode`) :`true` "ForDuration" :!type "EDrawDebugTrace Enum") :`DrawTime` 0.05))
        (if _returnvalue_3
          (set `self.BlockLeft` true)
          (else
            (set `self.BlockLeft` false))))
      (:`then_3`
        ;[1 1 1] Right
        (bind (_outhit_4 _returnvalue_4) (`KismetSystemLibrary.LineTraceSingleForObjects` :`Start` (`KismetMathLibrary.MakeVector` _returnvalue_x _returnvalue_y (+ _returnvalue_z 50.0)) :`End` (`KismetMathLibrary.MakeVector` _returnvalue_x_8 (+ _returnvalue_y_8 100.0) (+ _returnvalue_z_8 0.0)) :`ObjectTypes` (`|MakeArray` "ObjectTypeQuery1" "ObjectTypeQuery2" :!type "EObjectTypeQuery Enum") :`DrawDebugType` (select `bool` (`self.DebugMode`) :`true` "ForDuration" :!type "EDrawDebugTrace Enum") :`DrawTime` 0.05))
        (if _returnvalue_4
          (set `self.BlockRight` true)
          (else
            (set `self.BlockRight` false)))))))

(fn `CheckSurfaceBool`
  (if (`self.IsFall`)
    (`PrimitiveComponent.SetSimulatePhysics` (`self.StaticMesh`) true)))

(fn `HorzDirection`
  (returns (out :type "Float (double-precision)"))
  (return (`KismetMathLibrary.Conv_IntToDouble` (`self.horzAxis`))))

(fn `IsAlwaysSurface`
  (bind (_returnvalue_x _returnvalue_y) (`KismetMathLibrary.BreakVector` (`self.K2_GetActorLocation`)))
  (if (not (`self.IsFall`))
    (bind (_outhit _returnvalue) (`KismetSystemLibrary.LineTraceSingleForObjects` :`Start` (`KismetMathLibrary.MakeVector` (.x (`self.K2_GetActorLocation`)) (.y (`self.K2_GetActorLocation`)) (- (.z (`self.K2_GetActorLocation`)) 50.0)) :`End` (`KismetMathLibrary.MakeVector` _returnvalue_x _returnvalue_y -100.0) :`ObjectTypes` (`|MakeArray` "ObjectTypeQuery1" "ObjectTypeQuery2" :!type "EObjectTypeQuery Enum") :`DrawDebugType` (select `bool` (`self.DebugMode`) :`true` "Persistent" :!type "EDrawDebugTrace Enum")))
    (if (not _returnvalue)
      (set `self.IsFall` true))))

(fn `MoveTween`
  (locals (stepPerc :type "Float (double-precision)") (stepMax :type Integer :default 30))
  (bind _returnvalue (`KismetMathLibrary.MakeVector` (* (`self.HorzDirection`) -1.0) (`self.VertDirection`) 0.0))
  (bind _output_get (set `local.stepPerc` (/ 1.0 (`KismetMathLibrary.Conv_IntToDouble` (`local.stepMax`)))))
  (bind _returnvalue_2 (* _output_get 90.0))
  (`self.K2_SetActorLocationAndRotation` (+ (`KismetMathLibrary.RotateAngleAxis` (- (`self.K2_GetActorLocation`) (`self.PivotPoint`)) _returnvalue_2 _returnvalue) (`self.PivotPoint`)) (`KismetMathLibrary.ComposeRotators` (`self.K2_GetActorRotation`) (`KismetMathLibrary.RotatorFromAxisAndAngle` _returnvalue _returnvalue_2)))
  (if (>= (`self.StepCounts`) (- (`local.stepMax`) 1))
    (set `self.stepCount` 0)
    (`KismetSystemLibrary.K2_ClearTimer` null "MoveTween")
    (else
      (set `self.stepCount` (+ (`self.StepCounts`) 1)))))

(fn `PivotPoint`
  (returns (out :type "Vector Structure"))
  (return (`KismetMathLibrary.MakeVector` (+ (* (`self.VertDirection`) 50.0) (.x (`self.lastPos`))) (+ (.y (`self.lastPos`)) (* (`self.HorzDirection`) 50.0)) 0.0)))

(fn `ResetVelocity`
  (`PrimitiveComponent.SetAllPhysicsLinearVelocity` (`self.StaticMesh`) (0.0 0.0 0.0) false))

(fn `SetState`
  (params (horzAxis :type Integer) (vertAxis :type Integer) (lastPos :type "Vector Structure"))
  (set `self.horzAxis` horzAxis)
  (set `self.vertAxis` vertAxis)
  (set `self.lastPos` lastPos))

(fn `StartMoving`
  (params (horzAxis :type Integer) (vertAxis :type Integer))
  (if (not (`KismetSystemLibrary.K2_IsTimerActive` null "MoveTween"))
    (`self.SetState` horzAxis vertAxis (`self.K2_GetActorLocation`))
    (`KismetSystemLibrary.K2_SetTimer` null "MoveTween" 0.0166 true))
  (return))

(fn `StepCounts`
  (returns (out :type Integer))
  (return (`self.stepCount`)))

(fn `UserConstructionScript`)

(fn `VertDirection`
  (returns (out :type "Float (double-precision)"))
  (return (`KismetMathLibrary.Conv_IntToDouble` (`self.vertAxis`))))